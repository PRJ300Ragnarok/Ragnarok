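; Close-range enemy AI actor that makes melee attacks on the player (BP_Achaeus) and has its own health.
; Attack plays a melee montage and arms a HitOnce flag, so the weapon hitbox overlap subtracts Damage from the player's Health only once per attack.
; DealingDamage lowers CurrentHealth, refreshes the Enemy_Health widget bar and destroys the actor at zero.
; Tick shows the health bar only while the player is nearby.
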(event OnComponentBeginOverlap(WeaponHitBox)
  (params (OverlappedComponent :type Primitive%20Component%20Object%20Reference) (OtherActor :type Actor%20Object%20Reference) (OtherComp :type Primitive%20Component%20Object%20Reference) (OtherBodyIndex :type Integer) (bFromSweep :type Boolean) (SweepResult :type Hit%20Result%20Structure%20%28by%20ref%29))
  ;[1 1 1] Deal Damage To Player
  (Variables|Default|SetDamage (Variables|Default|GetDamage))
  (bind _outactors (Actor|GetAllActorsOfClass "/Game/Domas/Character/BP_Achaeus.BP_Achaeus_C"))
  (for _array_element _outactors
    (bind _output_get (Variables|Default|SetPlayer _array_element))
    (if (and (== _array_element (.HitActor (Collision|BreakHitResult SweepResult))) (Math|Boolean|Equal(Boolean) true (Variables|Default|GetHitOnce)))
      (Variables|/Game/Domas/Character/BP_Achaeus.BP_Achaeus_C|SetHealth _output_get (- (Variables|/Game/Domas/Character/BP_Achaeus.BP_Achaeus_C|GetHealth _output_get) (Math|Conversions|ToFloat(Integer) (Variables|Default|GetDamage))))
      (Variables|Default|SetHitOnce false))))

(event Custom|Attack
  ;[1 1 1] Animation
  (Variables|Default|SetHitOnce true)
  (Animation|Montage|PlayMontage (Variables|Character|GetMesh) "/Game/Domas/AI_Enemies/Animations/Melee_A_Montage.Melee_A_Montage"))

(event EventTick
  (params (DeltaSeconds :type Float%20%28single-precision%29))
  ;[1 1 1] Show Health
  (if (< (Transformation|GetDistanceTo (Game|GetPlayerCharacter 0)) 2e+03)
    (Rendering|SetVisibility (Variables|Default|GetEnemyHealth) true false)
    (else
      (Rendering|SetVisibility (Variables|Default|GetEnemyHealth) false false))))

(event EventBeginPlay
  ;[1 1 1] Lose HP
  (CallFunction|UpdateHealth))

(event EventDealingDamage
  (params (Damage :type Integer) (Sender :type Actor%20Object%20Reference))
  ;[1 1 1] Lose HP
  (Variables|Default|SetCurrentHealth (- (Variables|Default|GetCurrentHealth) Damage))
  (CallFunction|UpdateHealth)
  (if (<= (Variables|Default|GetCurrentHealth) 0)
    (Actor|DestroyActor)))

(fn ConstructionScript)

(fn UpdateHealth
  (bind _asenemy_health (Utilities|Casting|CastToEnemy_Health (UserInterface|GetUserWidgetObject (Variables|Default|GetEnemyHealth))))
  (Progress|SetPercent (Variables|/Game/Domas/AI_Enemies/Enemy_Health.Enemy_Health_C|GetHealth _asenemy_health) (/ (Math|Conversions|ToFloat(Integer) (Variables|Default|GetCurrentHealth)) (Math|Conversions|ToFloat(Integer) (Variables|Default|GetMaxHealth))))
  (return))