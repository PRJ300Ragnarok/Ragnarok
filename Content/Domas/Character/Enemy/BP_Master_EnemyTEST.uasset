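; BP_Master_EnemyTEST is a test master enemy Blueprint that tracks health and shows it on an Enemy_Health widget.
; On BeginPlay and on each DealingDamage event, it sets the widget's progress bar to current over max health.
; Damage subtracts from CurrentHealth, and only when it lands exactly on zero does it print "Dead" and play the Dying montage.
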(event EventBeginPlay
  (CallFunction|UpdateHealth))

(event EventDealingDamage
  (params (Damage :type Integer) (Sender :type Actor%20Object%20Reference))
  (Variables|Default|SetCurrentHealth (- (Variables|Default|GetCurrentHealth) Damage))
  (CallFunction|UpdateHealth)
  (if (== (Variables|Default|GetCurrentHealth) 0)
    (Development|PrintString "Dead")
    (Animation|PlayAnimMontage "/Game/Domas/Character/Animations/Dying.Dying" 1.0 "None")))

(fn ConstructionScript)

(fn UpdateHealth
  (bind _asenemy_health (Utilities|Casting|CastToEnemy_Health (UserInterface|GetUserWidgetObject (Variables|Default|GetEnemyHealth))))
  (Progress|SetPercent (Variables|/Game/Domas/AI_Enemies/Enemy_Health.Enemy_Health_C|GetHealth _asenemy_health) (/ (Math|Conversions|ToFloat(Integer) (Variables|Default|GetCurrentHealth)) (Math|Conversions|ToFloat(Integer) (Variables|Default|GetMaxHealth))))
  (return))