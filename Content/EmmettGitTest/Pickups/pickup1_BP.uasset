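; An inventory pickup actor whose mesh is chosen by an Index into a Meshes array in the construction script.
; When a BP_Achaeus actor overlaps it, it finds the first top-level Inventory widget and calls Additem with that Index.
; The pickup then destroys itself.
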(event EventBeginPlay)

(event EventTick
  (params (DeltaSeconds :type Float%20%28single-precision%29)))

(event Collision|EventActorBeginOverlap
  (params (OtherActor :type Actor%20Object%20Reference))
  (Utilities|Casting|CastToBP_Achaeus OtherActor)
  (bind _foundwidgets (Widget|GetAllWidgetsOfClass "/Game/EmmettGitTest/Pickups/inventory.inventory_C" true))
  (Default|Additem (Utilities|Array|Get(acopy) _foundwidgets) (Variables|Default|Getindex))
  (Actor|DestroyActor))

(fn ConstructionScript
  (Components|StaticMesh|SetStaticMesh (Variables|Default|GetStaticMesh) (Utilities|Array|Get(acopy) (Variables|Default|Getmeshes) (Variables|Default|Getindex))))